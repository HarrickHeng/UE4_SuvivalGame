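; Game instance that serves as the UI manager for a survival game, covering runtime HUD, message box, pickable, inventory, cabinet and failed screens.
; Events route through a shared ShowPanel, which lazily creates, caches and registers each widget, and HidePanel, which removes it.
; An active-panel counter switches to game-only input without cursor once modal panels close.
; MessagePush forwards text to the message box, while HideAllPanel removes every registered widget.
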(event `CreateRuntimeUI`
  (`self.ShowPanel` false (`self.RuntimeUI`) "/Game/UI/UI_Runtime.UI_Runtime_C" (`GameplayStatics.GetPlayerController` 0))
  (`self.ShowPanel` false (`self.MessageBoxPanel`) "/Game/UI/UI_MessageBox.UI_MessageBox_C" (`GameplayStatics.GetPlayerController` 0)))

(event `MessagePush`
  (params (ContentTxt :type String))
  (bind _messageboxpanel (`self.MessageBoxPanel`))
  (`/Engine/EditorBlueprintResources/StandardMacros.IsValid` _messageboxpanel
    (:`Is Valid`
      (if true
        (`/Game/UI/UI_MessageBox.AddMessage` _messageboxpanel ContentTxt)))))

(event `CreatePickablePanel`
  (`self.ShowPanel` true (`self.PickablePanel`) "/Game/UI/UI_PickablePanel.UI_PickablePanel_C" (`GameplayStatics.GetPlayerController` 0)))

(event `HidePickablePanel`
  (`self.HidePanel` (`self.PickablePanel`) (`GameplayStatics.GetPlayerController` 0)))

(event `CreateInventoryPanel`
  (`self.ShowPanel` true (`self.InventoryPanel`) "/Game/UI/UI_Inventory.UI_Inventory_C" (`GameplayStatics.GetPlayerController` 0)))

(event `HideInventoryPanel`
  (`self.HidePanel` (`self.InventoryPanel`) (`GameplayStatics.GetPlayerController` 0)))

(event `CreateCabinetUI`
  (`self.ShowPanel` true (`self.CabinetUI`) "/Game/UI/UI_Cabinet.UI_Cabinet_C" (`GameplayStatics.GetPlayerController` 0)))

(event `HideCabinetUI`
  (`self.HidePanel` (`self.CabinetUI`) (`GameplayStatics.GetPlayerController` 0)))

(event `CreateFailedUI`
  (`self.ShowPanel` true (`self.FailedPanel`) "/Game/UI/UI_Failed.UI_Failed_C" (`GameplayStatics.GetPlayerController` 0)))

(event `HIdeFaildedUI`
  (`self.HidePanel` (`self.FailedPanel`) (`GameplayStatics.GetPlayerController` 0)))

(event `HideAllPanel`
  (for _array_element (`self.UI_Array`)
    (`self.HidePanel` _array_element (`GameplayStatics.GetPlayerController` 0)))
  (`KismetArrayLibrary.Array_Clear` (`self.UI_Array`)))

(fn `HidePanel`
  (params (PanelTypeClass :type "UserWidget Object Reference") (PlayerController :type "PlayerController Object Reference"))
  (`/Engine/EditorBlueprintResources/StandardMacros.IsValid` PanelTypeClass
    (:`Is Valid`
      (`Widget.RemoveFromParent` PanelTypeClass)
      (bind _result (`/Engine/EditorBlueprintResources/StandardMacros.DecrementInt` (`self.ActiveUICount`))
        (:`  `
          (if (<= _result 0)
            (`WidgetBlueprintLibrary.SetInputMode_GameOnly` PlayerController)
            (set `PlayerController.bShowMouseCursor` false PlayerController)))))))

(fn `ShowPanel`
  (params (bChangeUIMode :type Boolean) (PanelVariable :type "UserWidget Object Reference (by ref)") (PanelTypeClass :type "UserWidget Class Reference") (PlayerController :type "PlayerController Object Reference"))
  (`/Engine/EditorBlueprintResources/StandardMacros.IsValid` PanelVariable
    (:`Is Valid`
      (if (not (`Widget.IsInViewport` PanelVariable))
        (`UserWidget.AddToViewport` PanelVariable 0 :!label _label)
        (if bChangeUIMode
          (`/Engine/EditorBlueprintResources/StandardMacros.IncrementInt` (`self.ActiveUICount`)
            (:`  `
              (`WidgetBlueprintLibrary.SetInputMode_GameAndUIEx` PlayerController PanelVariable)
              (set `PlayerController.bShowMouseCursor` true PlayerController)))
          (else
            (`WidgetBlueprintLibrary.SetInputMode_GameOnly` PlayerController)
            (set `PlayerController.bShowMouseCursor` false PlayerController)))))
    (:`Is Not Valid`
      (bind _returnvalue (`|CreateWidget` PanelTypeClass PlayerController))
      (`|VariableSetRef` PanelVariable _returnvalue)
      (`KismetArrayLibrary.Array_Add` (`self.UI_Array`) PanelVariable)
      (goto _label))))