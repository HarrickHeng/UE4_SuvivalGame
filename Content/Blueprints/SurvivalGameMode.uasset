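; Survival game mode that sets up the runtime UI and handles game over, restart and quit.
; On BeginPlay it caches the level's GlobalTimer and has the game instance create the runtime UI.
; Game over stops the timer, shows the failed panel and passes it the survived day and hour.
; CheckScore compares total hours survived against the bestScore save slot, saves new records and returns the result text.
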(event `self.ReceiveBeginPlay`
  (set `self.GameInstance` (cast `/Game/Blueprints/SurvivalGameInstance` (`GameplayStatics.GetGameInstance`) :!pure true))
  (bind _outactors (`GameplayStatics.GetAllActorsOfClass` "/Game/Blueprints/GlobalTimer.GlobalTimer_C"))
  (for _array_element _outactors
    (set `self.GlobalTimer` _array_element)
    (`/Game/Blueprints/SurvivalGameInstance.CreateRuntimeUI` (`self.GameInstance`))))

(event `GameOver`
  (bind _gameinstance (`self.GameInstance`))
  (bind _globaltimer (`self.GlobalTimer`))
  (bind _currentday (`/Game/Blueprints/GlobalTimer.CurrentDay` _globaltimer))
  (bind _currenthour (`/Game/Blueprints/GlobalTimer.CurrentHour` _globaltimer))
  (`/Game/Blueprints/GlobalTimer.StopTimer` (`self.GlobalTimer`))
  (`/Game/Blueprints/SurvivalGameInstance.HideAllPanel` (`self.GameInstance`))
  (`/Game/Blueprints/SurvivalGameInstance.CreateFailedUI` _gameinstance)
  (bind _recordtext (`self.CheckScore` _currentday _currenthour))
  (`/Game/UI/UI_Failed.SetTexts` (`/Game/Blueprints/SurvivalGameInstance.FailedPanel` _gameinstance) _currentday _currenthour _recordtext))

(event `RestartGame`
  (`GameplayStatics.OpenLevel` "MainLevel"))

(event `QuitGame`
  (`KismetSystemLibrary.ExecuteConsoleCommand` "exit" null))

(fn `CheckScore`
  (params (NewDay :type Integer) (NewHour :type Integer))
  (returns (RecordText :type String))
  (bind _returnvalue (`GameplayStatics.DoesSaveGameExist` "bestScore"))
  (if _returnvalue
    (bind _returnvalue_2 (`GameplayStatics.LoadGameFromSlot` "bestScore"))
    (bind _asbeat_score (cast `/Game/Blueprints/BeatScore` _returnvalue_2))
    (bind _bestday (`/Game/Blueprints/BeatScore.BestDay` _asbeat_score))
    (bind _besthour (`/Game/Blueprints/BeatScore.BestHour` _asbeat_score))
    (if (>= (+ (* NewDay 24) NewHour) (+ (* _bestday 24) _besthour))
      _
      (else
        (return (`KismetStringLibrary.Concat_StrStr` "目前最佳记录：" (`KismetStringLibrary.Conv_IntToString` _bestday) "天" (`KismetStringLibrary.Conv_IntToString` _besthour) "小时")))))
  (bind _returnvalue_3 (`GameplayStatics.CreateSaveGameObject` "/Game/Blueprints/BeatScore.BeatScore_C"))
  (set `/Game/Blueprints/BeatScore.BestDay` NewDay _returnvalue_3)
  (set `/Game/Blueprints/BeatScore.BestHour` NewHour _returnvalue_3)
  (`GameplayStatics.SaveGameToSlot` _returnvalue_3 "bestScore")
  (return "恭喜你创造了新纪录！"))

(fn `UserConstructionScript`)