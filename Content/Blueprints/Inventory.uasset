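; Weight-limited inventory that stacks item slots by name in the Content map.
; TryAddItem uses IsOverLoad to test class-default weight times count against MaxLoad, then updates Load, merges or inserts the slot, fires ChangeCount or AddItem dispatchers, and returns success with Chinese feedback text.
; RemoveItem decrements or deletes a slot, but neither lowers Load nor fires a dispatcher.
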(fn `IsOverLoad`
  (params (NewItem :type "/Game/Blueprints/Prop/ItemSlot Structure"))
  (returns (WillOverLoad :type Boolean) (NewLoad :type Integer))
  (bind (_type _name _icon _count) (break `/Game/Blueprints/Prop/ItemSlot` NewItem))
  (bind _returnvalue (+ (* (`.Weight` (defaults `Object` _type)) _count) (`self.Load`)))
  (return (> _returnvalue (`self.MaxLoad`)) _returnvalue))

(fn `RemoveItem`
  (params (RemoveItem :type "/Game/Blueprints/Prop/ItemSlot Structure"))
  (locals (NewItemSlot :type "/Game/Blueprints/Prop/ItemSlot Structure"))
  (bind (_type _name _icon _count) (break `/Game/Blueprints/Prop/ItemSlot` RemoveItem))
  (bind (_value _returnvalue) (`BlueprintMapLibrary.Map_Find` (`self.Content`) _name))
  (bind (_type_2 _name_2 _icon_2 _count_2) (break `/Game/Blueprints/Prop/ItemSlot` _value))
  (bind _returnvalue_2 (- _count_2 _count))
  (if _returnvalue
    (if (> _returnvalue_2 0)
      (set `local.NewItemSlot` (make `/Game/Blueprints/Prop/ItemSlot` _type_2 _name_2 _icon_2 _returnvalue_2))
      (`BlueprintMapLibrary.Map_Remove` (`self.Content`) _name)
      (`BlueprintMapLibrary.Map_Add` (`self.Content`) _name (`local.NewItemSlot`))
      (else
        (`BlueprintMapLibrary.Map_Remove` (`self.Content`) _name)))))

(fn `TryAddItem`
  (params (NewItem :type "/Game/Blueprints/Prop/ItemSlot Structure"))
  (returns (AddSuc :type Boolean) (FeedbackInfo :type String))
  (locals (TempItemSlot :type "/Game/Blueprints/Prop/ItemSlot Structure"))
  (bind (_type _name _icon _count) (break `/Game/Blueprints/Prop/ItemSlot` NewItem))
  (bind (_type_2 _name_2) (break `/Game/Blueprints/Prop/ItemSlot` NewItem))
  (bind (_type_3 _name_3 _icon_2 _count_2) (break `/Game/Blueprints/Prop/ItemSlot` (`BlueprintMapLibrary.Map_Find` (`self.Content`) _name)))
  (bind (_willoverload _newload) (`self.IsOverLoad` NewItem))
  (if _willoverload
    (return false "装不下这件物品，请清理背包！")
    (else
      (set `self.Load` _newload)
      (if (`BlueprintMapLibrary.Map_Contains` (`self.Content`) _name_2)
        (`self.ChangeCount` NewItem)
        (set `local.TempItemSlot` (make `/Game/Blueprints/Prop/ItemSlot` _type_3 _name_3 _icon_2 (+ _count_2 _count)))
        (`BlueprintMapLibrary.Map_Remove` (`self.Content`) _name)
        (`BlueprintMapLibrary.Map_Add` (`self.Content`) _name (`local.TempItemSlot`))
        (return true (`KismetStringLibrary.Concat_StrStr` "拾取了：" _name))
        (else
          (`BlueprintMapLibrary.Map_Add` (`self.Content`) _name_2 NewItem)
          (`self.AddItem` NewItem)
          (return true (`KismetStringLibrary.Concat_StrStr` "拾取了：" _name)))))))