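; Cabinet is a storage prop in a survival game that holds item stacks in a name-keyed map.
; Its overlap area shows or hides the cabinet UI through the game instance when a survival character enters or leaves, flagging the first player's state as near.
; AddItem and RemoveItem merge or reduce stacks by re-inserting map entries, deleting depleted ones.
; Both call added, updated-count or removed notifications carrying the item data.
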(event `self.AffectArea.OnComponentBeginOverlap`
  (params (OverlappedComponent :type "PrimitiveComponent Object Reference") (OtherActor :type "Actor Object Reference") (OtherComp :type "PrimitiveComponent Object Reference") (OtherBodyIndex :type Integer) (bFromSweep :type Boolean) (SweepResult :type "HitResult Structure (by ref)"))
  (cast `/Game/Mannequin/Character/SurvivalCharacter` OtherActor)
  (`/Game/Blueprints/SurvivalGameInstance.CreateCabinetUI` (cast `/Game/Blueprints/SurvivalGameInstance` (`GameplayStatics.GetGameInstance`) :!pure true))
  (set `/Game/Blueprints/SurvivalPlayerState.IsCabinetNear` true (cast `/Game/Blueprints/SurvivalPlayerState` (`Pawn.PlayerState` (`GameplayStatics.GetPlayerPawn` 0)) :!pure true)))

(event `self.AffectArea.OnComponentEndOverlap`
  (params (OverlappedComponent :type "PrimitiveComponent Object Reference") (OtherActor :type "Actor Object Reference") (OtherComp :type "PrimitiveComponent Object Reference") (OtherBodyIndex :type Integer))
  (bind _returnvalue (`GameplayStatics.GetPlayerPawn` 0))
  (cast `/Game/Mannequin/Character/SurvivalCharacter` OtherActor)
  (`/Game/Blueprints/SurvivalGameInstance.HideCabinetUI` (cast `/Game/Blueprints/SurvivalGameInstance` (`GameplayStatics.GetGameInstance`) :!pure true))
  (if (`KismetSystemLibrary.IsValid` _returnvalue)
    (set `/Game/Blueprints/SurvivalPlayerState.IsCabinetNear` false (cast `/Game/Blueprints/SurvivalPlayerState` (`Pawn.PlayerState` _returnvalue) :!pure true))))

(fn `AddItem`
  (params (NewItem :type "/Game/Blueprints/Prop/ItemSlot Structure"))
  (locals (name :type String) (count :type Integer))
  (bind (_type _name _icon _count) (break `/Game/Blueprints/Prop/ItemSlot` NewItem))
  (bind (_type_2 _name_2) (break `/Game/Blueprints/Prop/ItemSlot` NewItem))
  (bind (_type_3 _name_3 _icon_2) (break `/Game/Blueprints/Prop/ItemSlot` NewItem))
  (bind (_value _returnvalue) (`BlueprintMapLibrary.Map_Find` (`self.Content`) _name))
  (bind _itemslot (make `/Game/Blueprints/Prop/ItemSlot` _type_3 (`local.name`) _icon_2 (`local.count`)))
  (bind (_type_4 _name_4 _icon_3) (break `/Game/Blueprints/Prop/ItemSlot` _itemslot))
  (if (`BlueprintMapLibrary.Map_Contains` (`self.Content`) _name_2)
    (set `local.name` _name_2)
    (if _returnvalue
      (set `local.count` (+ (`.Count_11_EAA9457F4FD1E80D7E7E928C4E4D28EA` (break `/Game/Blueprints/Prop/ItemSlot` _value)) _count))
      (`BlueprintMapLibrary.Map_Remove` (`self.Content`) (`local.name`))
      (`BlueprintMapLibrary.Map_Add` (`self.Content`) (`local.name`) _itemslot)
      (`self.UpdatedItemCount` (make `/Game/Blueprints/Prop/ItemSlot` _type_4 _name_4 _icon_3 _count))
      (return))
    (else
      (`BlueprintMapLibrary.Map_Add` (`self.Content`) _name_2 NewItem)
      (`self.AddedItem` NewItem)
      (return))))

(fn `RemoveItem`
  (params (RemoveItem :type "/Game/Blueprints/Prop/ItemSlot Structure"))
  (locals (name :type String) (count :type Integer))
  (bind (_type _name _icon _count) (break `/Game/Blueprints/Prop/ItemSlot` RemoveItem))
  (bind (_type_2 _name_2 _icon_2 _count_2) (break `/Game/Blueprints/Prop/ItemSlot` RemoveItem))
  (bind _returnvalue (- (`.Count_11_EAA9457F4FD1E80D7E7E928C4E4D28EA` (break `/Game/Blueprints/Prop/ItemSlot` (`BlueprintMapLibrary.Map_Find` (`self.Content`) (`local.name`)))) _count))
  (set `local.name` _name)
  (set `local.count` _returnvalue)
  (if (`BlueprintMapLibrary.Map_Contains` (`self.Content`) (`local.name`))
    (if (> _returnvalue 0)
      (bind _returnvalue_2 (`BlueprintMapLibrary.Map_Remove` (`self.Content`) (`local.name`)))
      (if _returnvalue_2
        (`BlueprintMapLibrary.Map_Add` (`self.Content`) (`local.name`) (make `/Game/Blueprints/Prop/ItemSlot` _type (`local.name`) _icon (`local.count`)))
        (`self.RemovedItem` (make `/Game/Blueprints/Prop/ItemSlot` _type_2 _name_2 _icon_2 _count_2) :!label _label)
        (return))
      (else
        (`BlueprintMapLibrary.Map_Remove` (`self.Content`) (`local.name`))
        (goto _label)))))

(fn `UserConstructionScript`)