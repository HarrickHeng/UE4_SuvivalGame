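; GlobalTimer drives the survival game's day/night cycle, finding the level's sky light, directional sun and sky sphere at BeginPlay.
; Each gated Tick derives day, hour and minute from offset game time, rotates the sun and updates the sky sphere until StopTimer closes the gate.
; Sky lighting blends cubemaps by sun angle instead of costly recapturing.
; Crossing 06:00 or 18:00 pushes a dawn or nightfall message through SurvivalGameInstance.
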(event `self.ReceiveBeginPlay`
  (`|ExecutionSequence`
    (:`then_0`
      (bind _outactors (`GameplayStatics.GetAllActorsOfClass` "/Script/Engine.SkyLight"))
      (set `self.SkyLight` (`|GetArrayItem` _outactors)))
    (:`then_1`
      (bind _outactors_2 (`GameplayStatics.GetAllActorsOfClass` "/Script/Engine.DirectionalLight"))
      (set `self.SunLight` (`|GetArrayItem` _outactors_2)))
    (:`then_2`
      (bind _outactors_3 (`GameplayStatics.GetAllActorsOfClass` "/Engine/EngineSky/BP_Sky_Sphere.BP_Sky_Sphere_C"))
      (set `self.SkySphere` (`|GetArrayItem` _outactors_3)))))

(event `self.ReceiveTick`
  (params (DeltaSeconds :type "Float (single-precision)"))
  (bind _secondsperday (`self.SecondsPerDay`))
  (bind _secondsperday_2 (`self.SecondsPerDay`))
  (bind _returnvalue (/ _secondsperday_2 24.0))
  (bind _returnvalue_2 (+ (`KismetSystemLibrary.GetGameTimeInSeconds`) (/ _secondsperday_2 4.0)))
  (bind (_remainder _returnvalue_3) (`KismetMathLibrary.FMod` _returnvalue_2 _secondsperday_2))
  (bind (_remainder_2 _returnvalue_4) (`KismetMathLibrary.FMod` _remainder _returnvalue))
  (bind _returnvalue_5 (+ (* (/ (`KismetMathLibrary.FMod` _returnvalue_2 _secondsperday) _secondsperday) -360.0) 90.0))
  (`/Engine/EditorBlueprintResources/StandardMacros.Gate` false :!label _label
    (:`Exit`
      (`/Engine/EngineSky/BP_Sky_Sphere.UpdateSunDirection` (`self.SkySphere`))
      (`self.K2_SetActorRotation` (`self.SunLight`) (`KismetMathLibrary.MakeRotator` 0.0 _returnvalue_5) false)
      (`self.UpdateSunLight` _returnvalue_5) ; cubemap线性捕捉渲染天光环境
      (set `self.CurrentDay` _returnvalue_3)
      (bind _output_get (set `self.CurrentHour` _returnvalue_4))
      (set `self.CurrentMinute` (`.ReturnValue` (`KismetMathLibrary.FMod` _remainder_2 (/ _returnvalue 60.0))))
      (`|ExecutionSequence`
        (:`then_0`
          (if (`self.IsDayTime`)
            (bind _returnvalue_6 (and (< _output_get 18) (>= _output_get 6)))
            (if (not _returnvalue_6)
              (`self.EnterNightTime`))
            (elif _returnvalue_6
              (`self.EnterDayTime`))))
        (:`then_1`
          (set `self.IsDayTime` _returnvalue_6))))))

(event `EnterDayTime`
  (`/Game/Blueprints/SurvivalGameInstance.MessagePush` (cast `/Game/Blueprints/SurvivalGameInstance` (`GameplayStatics.GetGameInstance`) :!pure true) "天亮了"))

(event `StopTimer`
  (goto _label :!via `Close`))

(event `EnterNightTime`
  (`/Game/Blueprints/SurvivalGameInstance.MessagePush` (cast `/Game/Blueprints/SurvivalGameInstance` (`GameplayStatics.GetGameInstance`) :!pure true) "天黑了"))

(fn `UpdateSunLight`
  (params (LightDirection :type "Float (double-precision)"))
  (bind _returnvalue (`KismetMathLibrary.DegSin` LightDirection))
  (bind _lightcomponent (`SkyLight.LightComponent` (`self.SkyLight`)))
  (if (>= _returnvalue 0.0)
    (`SkyLightComponent.SetCubemapBlend` _lightcomponent "/Game/Textures/Morning.Morning" "/Game/Textures/NightNoon.NightNoon" _returnvalue :!pinned true) ; 日落
    (else
      (`SkyLightComponent.SetCubemapBlend` _lightcomponent "/Game/Textures/Morning.Morning" "/Game/Textures/Noon.Noon" (`KismetMathLibrary.Abs` _returnvalue)) ; 日出
    )))

(fn `UserConstructionScript`)